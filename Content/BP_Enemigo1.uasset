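; Enemy actor that flies straight along its initial forward vector and periodically fires from DisparoLugar.
; Each tick moves it and advances a fire timer, spawning one of four random enemy projectile types at its own rotation.
; Overlapping the player or a BalaMIa-tagged bullet fires OnEnemyDestroy, which reports a kill to BP_GameMode and destroys the actor after a short delay.
; Player contact also reports a hit to the GameMode.
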(event `self.ReceiveBeginPlay`
  (set `self.MovementVector` (`self.GetActorForwardVector`))
  (add `self.OnEnemyDestroy` (delegate `DestroyedEvent`)))

(event `DestroyedEvent`
  (bind _asbp_game_mode (cast `/Game/BP_GameMode` (`GameplayStatics.GetGameMode`)))
  (`/Game/BP_GameMode.EnemigoMatado` _asbp_game_mode)
  (`KismetSystemLibrary.Delay` 0.1)
  (`self.K2_DestroyActor`))

(event `self.ReceiveActorBeginOverlap`
  (params (OtherActor :type "Actor Object Reference"))
  (if (`KismetArrayLibrary.Array_Contains` (`Actor.Tags` OtherActor) "Player")
    (`self.OnEnemyDestroy`)
    (bind _asbp_game_mode (cast `/Game/BP_GameMode` (`GameplayStatics.GetGameMode`)))
    (`/Game/BP_GameMode.HasSidoGolpeado` _asbp_game_mode)
    (elif (`KismetArrayLibrary.Array_Contains` (`Actor.Tags` OtherActor) "BalaMIa")
      (`self.OnEnemyDestroy`))))

(event `self.ReceiveTick`
  (params (DeltaSeconds :type "Float (single-precision)"))
  (`self.Moverse` DeltaSeconds)
  (bind _output_get (set `self.ShootCurrentTime` (+ DeltaSeconds (`self.ShootCurrentTime`))))
  (if (> _output_get (`self.DelayShoot`))
    (set `self.ShootCurrentTime` 0.0)
    (`self.Disparar`)))

(fn `Disparar`
  (bind _disparoelegido (`self.ElegirMunicion`))
  (bind _returnvalue (`|SpawnActorFromClass` _disparoelegido (`SceneComponent.K2_GetComponentToWorld` (`self.DisparoLugar`)) "Undefined" "MultiplyWithRoot" null null))
  (`self.K2_SetActorRotation` _returnvalue (`self.K2_GetActorRotation`) false))

(fn `ElegirMunicion`
  (returns (DisparoElegido :type "Actor Class Reference"))
  (return (select `int` (`KismetMathLibrary.RandomInteger` 4) :`0` "/Game/BP_DisparoEnemigo.BP_DisparoEnemigo_C" :`1` "/Game/BP_DisparoEnemigoFuribundo.BP_DisparoEnemigoFuribundo_C" :`2` "/Game/BP_DisparoEnemigoDorado.BP_DisparoEnemigoDorado_C" :`3` "/Game/BP_DisparoEnemigoVengatulivo.BP_DisparoEnemigoVengatulivo_C" :!type "Actor Class Reference")))

(fn `Moverse`
  (params (DeltaTime :type "Float (double-precision)"))
  (`self.K2_SetActorLocation` (+ (`self.K2_GetActorLocation`) (* (* DeltaTime (`self.Speed`)) (`self.MovementVector`)))))

(fn `UserConstructionScript`)