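; Game mode for a ship game that tracks kill progress and world number, and relays gameplay events to the player ship and HUD.
; EnemigoMatado increments Progress and, every tenth count (first at nine), advances Mundo and calls EnemigoMurio on BP_HUD.
; HasSidoGolpeado forwards damage to BP_PlayerNave, and Muerte tells the HUD the player died, both through casts on player index 0.
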(event `EnemigoMatado`
  (bind _returnvalue (+ (`self.Progress`) 1))
  (set `self.Progress` _returnvalue)
  (if (== (mod _returnvalue 10) 0)
    (set `self.Mundo` (+ (`self.Mundo`) 1))
    (bind _asbp_hud (cast `/Game/BP_HUD` (`PlayerController.GetHUD` (`GameplayStatics.GetPlayerController` 0))))
    (`/Game/BP_HUD.EnemigoMurio` _asbp_hud)))

(event `HasSidoGolpeado`
  (bind _asbp_player_nave (cast `/Game/BP_PlayerNave` (`GameplayStatics.GetPlayerPawn` 0)))
  (`/Game/BP_PlayerNave.RecibirDanio` _asbp_player_nave))

(event `self.ReceiveTick`
  (params (DeltaSeconds :type "Float (single-precision)")))

(event `Muerte`
  (bind _asbp_hud (cast `/Game/BP_HUD` (`PlayerController.GetHUD` (`GameplayStatics.GetPlayerController` 0))))
  (`/Game/BP_HUD.JugadorMuerto` _asbp_hud))

(fn `UserConstructionScript`)