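; BP_DisparoEnemigo is an enemy projectile that travels in a straight line and reports hits on the player ship.
; Tick moves it along its forward vector at Speed, scaled by delta time and without sweep.
; On overlap with BP_PlayerNave it calls HasSidoGolpeado on BP_GameMode, then destroys itself after a tiny delay.
; Overlapping an actor tagged MuroBala also destroys it after the same delay.
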(event `self.ReceiveActorBeginOverlap`
  (params (OtherActor :type "Actor Object Reference"))
  (cast `/Game/BP_PlayerNave` OtherActor
    (:`then`
      (bind _asbp_game_mode (cast `/Game/BP_GameMode` (`GameplayStatics.GetGameMode`)))
      (`/Game/BP_GameMode.HasSidoGolpeado` _asbp_game_mode)
      (`KismetSystemLibrary.Delay` 0.01)
      (`self.K2_DestroyActor`))
    (:`CastFailed`
      (if (`KismetArrayLibrary.Array_Contains` (`Actor.Tags` OtherActor) "MuroBala")
        (`KismetSystemLibrary.Delay` 0.01)
        (`self.K2_DestroyActor`)))))

(event `self.ReceiveTick`
  (params (DeltaSeconds :type "Float (single-precision)"))
  (`self.K2_SetActorLocation` (+ (`self.K2_GetActorLocation`) (* (`self.GetActorForwardVector`) (* DeltaSeconds (`self.speed`))))))

(fn `UserConstructionScript`)