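; BP_Spawner2 is an enemy spawner that creates BP_Enemigo2 actors on a repeating timer.
; BeginPlay starts a looping timer at SpawnTime and caches BP_GameMode.
; Each tick of that timer calls SpawnEnemigos, which spawns at a randomly chosen scene component tagged "Spawners".
; GetClassToSpawn maps a clamped world index to an enemy class, but the spawn call hardcodes BP_Enemigo2 instead of using it.
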(event `self.ReceiveBeginPlay`
  (`KismetSystemLibrary.K2_SetTimerDelegate` (delegate `SpawnEnemy`) (`self.SpawnTime`) true)
  (bind _asbp_game_mode (cast `/Game/BP_GameMode` (`GameplayStatics.GetGameMode`)))
  (set `self.GameModeNave` _asbp_game_mode))

(event `SpawnEnemy`
  (`self.SpawnEnemigos`))

(fn `GetClassToSpawn`
  (params (Mundo :type Integer))
  (returns (EnemigoSeleccionado :type "Actor Class Reference"))
  (return (select `int` (`KismetMathLibrary.Clamp` Mundo 0 (- (`self.NumEnemigosMax`) 1)) :`0` "/Game/BP_Enemigo1.BP_Enemigo1_C" :`1` "/Game/BP_Enemigo2.BP_Enemigo2_C" :`2` "/Game/BP_Enemigo2.BP_Enemigo2_C" :!type "Actor Class Reference")))

(fn `SpawnEnemigos`
  (bind _returnvalue (`self.GetComponentsByTag` "/Script/Engine.SceneComponent" "Spawners"))
  (`|SpawnActorFromClass` "/Game/BP_Enemigo2.BP_Enemigo2_C" (`SceneComponent.K2_GetComponentToWorld` (`|GetArrayItem` _returnvalue (`KismetMathLibrary.RandomInteger` (`KismetArrayLibrary.Array_Length` _returnvalue)))) "Undefined" "MultiplyWithRoot" null null))

(fn `UserConstructionScript`)