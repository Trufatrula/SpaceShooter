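; BP_PlayerNave is the player ship pawn, moved and fired through Enhanced Input, with a lives count.
; On BeginPlay it adds its mapping context; move input feeds movement along its right and forward vectors and prints the X value.
; Firing spawns the Municion class at PuntoDisparo, gated by CanFire and a cooldown timer.
; RecibirDanio removes a life and calls Muerte on BP_GameMode when Vidas reaches zero.
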(event `self.ReceiveBeginPlay`
  (bind _asplayer_controller (cast `PlayerController` (`self.GetController`)))
  (bind _returnvalue (pcsubsystem `EnhancedInputLocalPlayerSubsystem` _asplayer_controller))
  (`/Engine/EditorBlueprintResources/StandardMacros.IsValid` _returnvalue
    (:`Is Valid`
      (`EnhancedInputSubsystemInterface.AddMappingContext` _returnvalue "/Game/Input_Mapping.Input_Mapping" 0 (struct)))))

(event `EnhancedInput|/Game/Input_Mover`
  (params (ActionValue :type "Vector2D Structure") (ElapsedSeconds :type "Float (double-precision)") (TriggeredSeconds :type "Float (double-precision)") (InputAction :type "InputAction Object Reference" :default "/Game/Input_Mover.Input_Mover"))
  (:`Triggered`
    (`KismetSystemLibrary.PrintString` (`KismetStringLibrary.Conv_DoubleToString` ActionValue_X))
    (`self.AddMovementInput` (`self.GetActorRightVector`) ActionValue_X)
    (`self.AddMovementInput` (`self.GetActorForwardVector`) ActionValue_Y)))

(event `EnhancedInput|/Game/Input_Disparo`
  (params (ActionValue :type Boolean) (ElapsedSeconds :type "Float (double-precision)") (TriggeredSeconds :type "Float (double-precision)") (InputAction :type "InputAction Object Reference" :default "/Game/Input_Disparo.Input_Disparo"))
  (:`Triggered`
    (if (`self.CanFire`)
      (`self.Disparar`)
      (set `self.CanFire` false)
      (`KismetSystemLibrary.K2_SetTimerDelegate` (delegate `CanFireAgain`) (`self.Cooldown`)))))

(event `CanFireAgain`
  (set `self.CanFire` true))

(event `RecibirDanio`
  (bind _output_get (set `self.Vidas` (- (`self.Vidas`) 1)))
  (if (== _output_get 0)
    (bind _asbp_game_mode (cast `/Game/BP_GameMode` (`GameplayStatics.GetGameMode`)))
    (`/Game/BP_GameMode.Muerte` _asbp_game_mode)))

(fn `Disparar`
  (`|SpawnActorFromClass` (`self.Municion`) (`SceneComponent.K2_GetComponentToWorld` (`self.PuntoDisparo`)) "Undefined" "MultiplyWithRoot" null null))

(fn `UserConstructionScript`)